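; BP_RockEnemy is an AI enemy whose attack is a one-time radial damage burst that also kills it.
; On BeginPlay it runs BT_RockEnemy with the player's pawn as blackboard Target, then mirrors IsDead to the blackboard every Tick.
; Attack, gated by animation state and death, deals random damage within the Sphere radius, zeroes Health, marks itself dead and updates the animation.
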(event EventBeginPlay
  (bind _returnvalue (AI|GetAIController self))
  (AI|RunBehaviorTree _returnvalue "/Game/Blueprints/BT_RockEnemy.BT_RockEnemy")
  (AI|Components|Blackboard|SetValueasObject (AI|GetBlackboard _returnvalue) (Utilities|Name|MakeLiteralName "Target") (Pawn|GetControlledPawn (Game|GetPlayerController 0)))
  (|CallParentFunction))

(event Collision|EventActorBeginOverlap
  (params (OtherActor :type Actor%20Object%20Reference)))

(event EventTick
  (params (DeltaSeconds :type Float%20%28single-precision%29))
  (bind _returnvalue (AI|GetAIController self))
  (AI|Components|Blackboard|SetValueasBool (AI|GetBlackboard _returnvalue) (Utilities|Name|MakeLiteralName "isDead?") (Variables|Default|GetisDead?))
  (|CallParentFunction DeltaSeconds))

(event EventAttack
  (if (Math|Boolean|ANDBoolean (Utilities|Enum|NotEqual(Enum) (Variables|Default|GetCurrentAnimState) "NewEnumerator4") (Utilities|Enum|NotEqual(Enum) (Variables|Default|GetCurrentAnimState) "NewEnumerator5") (not (Variables|Default|GetisDead?)) (Utilities|Enum|NotEqual(Enum) (Variables|Default|GetCurrentAnimState) "NewEnumerator2"))
    (Utilities|FlowControl|DoOnce false
      (:Completed
        (Variables|Default|SetCurrentAnimState "NewEnumerator3")
        (Game|Damage|ApplyRadialDamage (Math|Conversions|ToFloat(Integer) (Math|Random|RandomIntegerinRange (Variables|Default|GetMinDamage) (Variables|Default|GetMaxDamage))) (Transformation|GetActorLocation) (Variables|/Script/Engine.SphereComponent|GetSphereRadius (Variables|Default|GetSphere)) "/Engine/EngineDamageTypes/DmgTypeBP_Environmental.DmgTypeBP_Environmental_C" 0 self 0 true "ECC_Visibility")
        (Variables|Default|SetHealth 0)
        (Variables|Default|SetisDead? true)
        (CallFunction|SetLooping false)
        (CallFunction|UpdateAnimation)))))

(fn ConstructionScript)