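; SpawnArea is a placeable actor that populates a box volume with a set number of actors of a configurable character class.
; The construction script sizes the box component from the AreaExtents variable.
; On BeginPlay, it loops NumObjects times, spawning at random offsets within the box extents around the actor's location using a random stream.
; Spawns adjust for collisions where possible but always spawn.
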(event EventBeginPlay
  (bind _stream (Variables|Default|GetStream))
  (bind _spawnarea (Variables|Default|GetSpawnArea))
  (bind _boxextent (Variables|/Script/Engine.BoxComponent|GetBoxExtent _spawnarea))
  (for _index (range 1 (Variables|Default|GetNumObjects))
    (Game|SpawnActorfromClass (Variables|Default|GetCharacterClassToSPawn) (Math|Transform|MakeTransform (+ (Math|Vector|MakeVector (Math|Random|RandomFloatinRangefromStream (* (.x _boxextent) -1.0) (.x _boxextent) _stream) (Math|Random|RandomFloatinRangefromStream (* (.y _boxextent) -1.0) (.y _boxextent) _stream) (Math|Random|RandomFloatinRangefromStream (* (.z _boxextent) -1.0) (.z _boxextent) _stream)) (Transformation|GetActorLocation)) "0, 0, 0" "1,1,1") "AdjustIfPossibleButAlwaysSpawn" 0 0)))

(event Collision|EventActorBeginOverlap
  (params (OtherActor :type Actor%20Object%20Reference)))

(event EventTick
  (params (DeltaSeconds :type Float%20%28single-precision%29)))

(fn ConstructionScript
  (Components|Box|SetBoxExtent (Variables|Default|GetSpawnArea) (Variables|Default|GetAreaExtents) true))