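; Base Paper2D side-scrolling character with run, jump and attack input, using water character flipbooks.
; Input sets CurrentPlayerState, while Tick returns Attacking to Idle near the flipbook's end and Jumping to Idle when no longer falling.
; Tick also yaws the controller to face X velocity and selects the flipbook from the state.
; Damage only prints a message, Running never resets to Idle by itself, and MoveRight's OR guard always passes.
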(event EventTick
  (params (DeltaSeconds :type Float%20%28single-precision%29))
  (bind _sprite (Variables|Default|GetSprite))
  (CallFunction|SpriteOrientationCheck)
  (Utilities|FlowControl|Sequence
    (:then_0
      (switch Utilities|FlowControl|Switch|SwitchonE_PlayerState (Variables|Default|GetCurrentPlayerState)
        (:NewEnumerator2
          (if (>= (/ (Components|Timeline|GetPlaybackPosition _sprite) (Class|PaperFlipbookComponent|GetFlipbookLength _sprite)) 0.9)
            (Variables|Default|SetCurrentPlayerState "NewEnumerator0")))
        (:NewEnumerator4
          (if (not (AI|Components|NavMovement|IsFalling (Variables|Character|GetCharacterMovement)))
            (Variables|Default|SetCurrentPlayerState "NewEnumerator0")))))
    (:then_1
      (CallFunction|UpdateAnimation))))

(event Game|Damage|EventAnyDamage
  (params (Damage :type Float%20%28single-precision%29) (DamageType :type Damage%20Type%20Object%20Reference) (InstigatedBy :type Controller%20Object%20Reference) (DamageCauser :type Actor%20Object%20Reference))
  (Development|PrintString (Utilities|String|Append "Taking " (Utilities|String|ToString(Float) Damage) " damage!")))

(event Input|ActionEvents|InputActionAttack
  (params (Key :type Key%20Structure :default "AnyKey"))
  (:Pressed
    (if (Utilities|Enum|NotEqual(Enum) (Variables|Default|GetCurrentPlayerState) "NewEnumerator4")
      (Variables|Default|SetCurrentPlayerState "NewEnumerator2")))
  (:Released
    (if (Utilities|Enum|NotEqual(Enum) (Variables|Default|GetCurrentPlayerState) "NewEnumerator4")
      (Variables|Default|SetCurrentPlayerState "NewEnumerator0"))))

(event Input|ActionEvents|InputActionJump
  (params (Key :type Key%20Structure :default "AnyKey"))
  (:Pressed
    (Variables|Default|SetCurrentPlayerState "NewEnumerator4")
    (Character|Jump)))

(event Input|AxisEvents|InputAxisMoveRight
  (params (AxisValue :type Float%20%28single-precision%29))
  (if (or (Utilities|Enum|NotEqual(Enum) (Variables|Default|GetCurrentPlayerState) "NewEnumerator2") (Utilities|Enum|NotEqual(Enum) (Variables|Default|GetCurrentPlayerState) "NewEnumerator4"))
    (if (> AxisValue 0.0)
      (Variables|Default|SetisMovingRight? true)
      (Pawn|Input|AddMovementInput "1.000000, 0, 0" AxisValue false :!label _label)
      (Variables|Default|SetCurrentPlayerState "NewEnumerator1")
      (elif (< AxisValue 0.0)
        (Variables|Default|SetisMovingRight? false)
        (goto _label)))))

(fn ConstructionScript)

(fn UpdateAnimation
  (Sprite|SetFlipbook (Variables|Default|GetSprite) (Utilities|Select :Index (Variables|Default|GetCurrentPlayerState) :NewEnumerator0 "/Game/Sprites/Flipbooks/FB_WaterCharacter_Idle.FB_WaterCharacter_Idle" :NewEnumerator1 "/Game/Sprites/Flipbooks/FB_WaterCharacter_Run.FB_WaterCharacter_Run" :NewEnumerator2 "/Game/Sprites/Flipbooks/FB_WaterCharacter_Attack.FB_WaterCharacter_Attack" :NewEnumerator4 "/Game/Sprites/Flipbooks/FB_WaterCharacter_Jump.FB_WaterCharacter_Jump" :NewEnumerator3 0)))

(fn SpriteOrientationCheck
  (Math|Float|CompareFloat (.X (Math|Vector|BreakVector (Variables|/Script/Engine.MovementComponent|GetVelocity (Pawn|GetMovementComponent)))) 0.0
    (:>
      (Pawn|SetControlRotation (Pawn|GetController) (Math|Rotator|MakeRotator 0.0 0.0 0.0)))
    (:<
      (Pawn|SetControlRotation (Pawn|GetController) (Math|Rotator|MakeRotator 0.0 0.0 1.8e+02)))))