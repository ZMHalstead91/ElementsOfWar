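; Player controller that creates the player HUD and shows a running play timer on it.
; On BeginPlay it spawns a W_PlayerHud widget, stores the reference and adds it to the viewport.
; Every Tick it adds DeltaSeconds to PlayTime and writes a minutes:seconds string straight into the HUD's TimeText, with only the minutes floored.
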(event EventBeginPlay
  (bind _returnvalue (UserInterface|CreateWidget "/Game/UI/W_PlayerHud.W_PlayerHud_C" self))
  (bind _output_get (Variables|Default|SetPHud_Ref _returnvalue))
  (UserInterface|Viewport|AddtoViewport _output_get 0))

(event EventTick
  (params (DeltaSeconds :type Float%20%28single-precision%29))
  (bind _output_get (Variables|Default|SetPlayTime (+ (Variables|Default|GetPlayTime) DeltaSeconds)))
  (Variables|/Game/UI/W_PlayerHud.W_PlayerHud_C|SetTimeText (Variables|Default|GetPHud_Ref) (Utilities|Text|FormatText "{Minutes}:{Seconds}" (Math|Float|Floor (/ _output_get 6e+01)) (Math|Float|%(Float) _output_get 6e+01))))

(fn ConstructionScript)